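; BP_Ball is a bouncing ball, apparently for a Breakout-style game, that detects misses.
; Each tick it moves along its normalized Direction at Speed using a swept SetActorLocation, scaled by delta time.
; On a hit it mirrors Direction around the surface normal and plays a knock sound.
; When its sphere overlaps a component tagged MissArea, it calls MissCount on BP_GameManager and destroys itself.
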(event OnComponentBeginOverlap(Sphere)
  (params (OverlappedComponent :type Primitive%20Component%20Object%20Reference) (OtherActor :type Actor%20Object%20Reference) (OtherComp :type Primitive%20Component%20Object%20Reference) (OtherBodyIndex :type Integer) (bFromSweep :type Boolean) (SweepResult :type Hit%20Result%20Structure%20%28by%20ref%29))
  ;[0.15 0.15 0.15 0.5] ゲームオーバー
  (if (Components|ComponentHasTag OtherComp "MissArea")
    (bind _returnvalue (Actor|GetActorOfClass "/Game/BP_GameManager.BP_GameManager_C"))
    (Default|MissCount _returnvalue)
    (Actor|DestroyActor)))

(event EventBeginPlay)

(event Collision|EventActorBeginOverlap
  (params (OtherActor :type Actor%20Object%20Reference)))

(event EventTick
  (params (DeltaSeconds :type Float%20%28single-precision%29))
  ;[0.15 0.15 0.15 0.5] 移動用
  (Transformation|SetActorLocation (+ (Transformation|GetActorLocation) (* (* (Math|Vector|Normalize (Variables|Default|GetDirection)) (Variables|Default|GetSpeed)) (Utilities|Time|GetWorldDeltaSeconds))) true false))

(event Collision|EventHit
  (params (MyComp :type Primitive%20Component%20Object%20Reference) (Other :type Actor%20Object%20Reference) (OtherComp :type Primitive%20Component%20Object%20Reference) (bSelfMoved :type Boolean) (HitLocation :type Vector :default "0, 0, 0") (HitNormal :type Vector :default "0, 0, 0") (NormalImpulse :type Vector :default "0, 0, 0") (Hit :type Hit%20Result%20Structure%20%28by%20ref%29))
  ;[0.15 0.15 0.15 0.5] 跳ね返り処理
  (Variables|Default|SetDirection (Math|Vector|MirrorVectorbyNormal (Variables|Default|GetDirection) HitNormal))
  (Audio|PlaySound2D "/Game/Breakout_SE_Knock.Breakout_SE_Knock" 1.0 1.0 0.0 0 0))

(fn ConstructionScript)
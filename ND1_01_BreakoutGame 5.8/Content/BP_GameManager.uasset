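; Game manager for a Breakout game that tracks blocks, remaining balls and the clear and game-over states.
; Block counters show the clear widget when none remain; a miss with no balls left shows game over unless cleared.
; Action reloads the level after game over, opens the next level after a clear, or otherwise spawns one ball at a time.
; The game instance carries the ball count, plus one bonus, between levels.
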(event EventBeginPlay
  (bind _asbpi_breakout_game_instance (Utilities|Casting|CastToBPI_BreakoutGameInstance (Game|GetGameInstance)))
  (bind _isvalidballnum (Default|IsValidBallNum _asbpi_breakout_game_instance))
  (if _isvalidballnum
    (Variables|Default|SetLeftBallNum (Variables|/Game/BPI_BreakoutGameInstance.BPI_BreakoutGameInstance_C|GetLeftBallNum _asbpi_breakout_game_instance))))

(event Collision|EventActorBeginOverlap
  (params (OtherActor :type Actor%20Object%20Reference)))

(event EventTick
  (params (DeltaSeconds :type Float%20%28single-precision%29)))

(fn ConstructionScript)

(fn AddBlockNum
  (bind _output_get (Variables|Default|SetBlockNum (+ (Variables|Default|GetBlockNum) 1)))
  (Development|PrintString (Utilities|String|Append "AddBlockNum :" (Utilities|String|ToString(Integer) _output_get))))

(fn AddBrokenBlockNum
  (bind _output_get (Variables|Default|SetBrokenBlockNum (+ (Variables|Default|GetBrokenBlockNum) 1)))
  (Development|PrintString (Utilities|String|Append "BrokenBlockNum :" (Utilities|String|ToString(Integer) _output_get)) true true "(R=0.000000,G=0.165492,B=1.000000,A=1.000000)")
  (bind _leftblocknum (CallFunction|GetLeftBlockNum))
  (Development|PrintString (Utilities|String|Append "LeftBlockNum :" (Utilities|String|ToString(Integer) _leftblocknum)) true true "(R=0.069232,G=0.000000,B=1.000000,A=1.000000)")
  (bind _leftblocknum_2 (CallFunction|GetLeftBlockNum))
  (if (== _leftblocknum_2 0)
    (CallFunction|ViewClearWidget)
    (Variables|Default|SetIsCleard true)))

(fn GetLeftBlockNum
  (return (- (Variables|Default|GetBlockNum) (Variables|Default|GetBrokenBlockNum))) ; リターンノードの入力ピンに\n返り値としたい値を入力すれば、\n関数の実行時に値が返ってくる
)

(fn ViewClearWidget
  (bind _returnvalue (UserInterface|CreateWidget "/Game/WBP_ClearWidget.WBP_ClearWidget_C"))
  (UserInterface|Viewport|AddtoViewport _returnvalue 0))

(fn ViewGameOverWidget
  (bind _returnvalue (UserInterface|CreateWidget "/Game/WBP_GameOverWidget.WBP_GameOverWidget_C"))
  (UserInterface|Viewport|AddtoViewport _returnvalue 0))

(fn MissCount
  ;[0.15 0.15 0.15 0.5] ゲームオーバー表示
  (Variables|Default|SetIsBallSpawned false) ; ボールの生成制限
  (if (and (<= (Variables|Default|GetLeftBallNum) 0) (not (Variables|Default|GetIsCleard)))
    (CallFunction|ViewGameOverWidget)
    (Variables|Default|SetIsGameOver true)))

(fn SpawnBall
  ;[0.15 0.15 0.15 0.5] ボールの動的生成
  (if (and (> (Variables|Default|GetLeftBallNum) 0) (not (Variables|Default|GetIsBallSpawned)))
    (Game|SpawnActorfromClass "/Game/BP_Ball.BP_Ball_C" (Math|Transform|MakeTransform (Transformation|GetActorLocation (Variables|Default|GetSpawnLocationActor))) "Undefined" "MultiplyWithRoot" 0 0) ; アクタを動的に生成するノード。生成するClassと\n生成する位置や向きや大きさ、アクタの生成時に十分な空間が\nなかったときの挙動などが設定できる。
    (Variables|Default|SetIsBallSpawned true)
    (Variables|Default|SetLeftBallNum (- (Variables|Default|GetLeftBallNum) 1))))

(fn Action
  (if (Variables|Default|GetIsGameOver) ; リセットの判断
    (CallFunction|LevelReset) ; レベルのリセット
    (elif (Variables|Default|GetIsCleard) ; レベルを上げるか、\nボールをスポーンさせる
      (CallFunction|OpenNextLevel) ; 次のレベルへ
      (else
        (CallFunction|SpawnBall) ; ボールのリスポーン可能状態へ
      ))))

(fn GetLeftBallNum
  ;[0.15 0.15 0.15 0.5] 残ボール数の取得用
  (return (Variables|Default|GetLeftBallNum)))

(fn LevelReset
  (bind _returnvalue (Game|GetCurrentLevelName true)) ; 現在開いているレベルの\n名前を取得する
  (Game|OpenLevel(byName) (Utilities|String|StringToName _returnvalue)) ; 指定した名前のレベルを開く
)

(fn OpenNextLevel
  (bind _asbpi_breakout_game_instance (Utilities|Casting|CastToBPI_BreakoutGameInstance (Game|GetGameInstance)))
  (Variables|/Game/BPI_BreakoutGameInstance.BPI_BreakoutGameInstance_C|SetLeftBallNum _asbpi_breakout_game_instance (+ (Variables|Default|GetLeftBallNum) 1))
  (Game|OpenLevel(byName) (Variables|Default|GetNextLevelName)))